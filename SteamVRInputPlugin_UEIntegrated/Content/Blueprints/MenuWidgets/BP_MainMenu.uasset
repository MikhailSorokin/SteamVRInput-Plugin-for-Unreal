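; BP_MainMenu is the main menu actor, hosting the left, lobby, matchmaking status, friends list and rankings panels as widget components.
; On BeginPlay it adds each component to PanelList and caches its typed CD widget, stopping at the first failed cast.
; It then passes itself to the game instance's global menu panel manager to instantiate it.
; Actor cursor events maintain a CursorOver flag.
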(event MouseInput|EventActorBeginCursorOver
  (Variables|Default|SetCursorOver true))

(event EventBeginPlay
  (bind _matchmakingstatuscomponent (Variables|Default|GetMatchmakingStatusComponent))
  (bind _friendslistwidgetcomponent (Variables|Default|GetFriendsListWidgetComponent))
  (bind _rankingswidgetcomponent (Variables|Default|GetRankingsWidgetComponent))
  (bind _leftwidgetcomponent (Variables|Default|GetLeftWidgetComponent))
  (bind _lobbywidgetcomponent (Variables|Default|GetLobbyWidgetComponent))
  (Utilities|Array|Add (Variables|Default|GetPanelList) _leftwidgetcomponent)
  (bind _ascdleft_widget (Utilities|Casting|CastToCDLeftWidget (UserInterface|GetUserWidgetObject _leftwidgetcomponent)))
  (Variables|Default|SetLeftPanel _ascdleft_widget)
  (Utilities|Array|Add (Variables|Default|GetPanelList) _lobbywidgetcomponent)
  (bind _ascdlobby_widget (Utilities|Casting|CastToCDLobbyWidget (UserInterface|GetUserWidgetObject _lobbywidgetcomponent)))
  (Variables|Default|SetLobbyPanel _ascdlobby_widget)
  (Utilities|Array|Add (Variables|Default|GetPanelList) _matchmakingstatuscomponent)
  (bind _ascdmatchmaking_status_widget (Utilities|Casting|CastToCDMatchmakingStatusWidget (UserInterface|GetUserWidgetObject _matchmakingstatuscomponent)))
  (Variables|Default|SetMatchmakingStatusPanel _ascdmatchmaking_status_widget)
  (Utilities|Array|Add (Variables|Default|GetPanelList) _friendslistwidgetcomponent)
  (bind _ascdfriends_list_widget (Utilities|Casting|CastToCDFriendsListWidget (UserInterface|GetUserWidgetObject _friendslistwidgetcomponent)))
  (Variables|Default|SetFriendsListPanel _ascdfriends_list_widget)
  (Utilities|Array|Add (Variables|Default|GetPanelList) _rankingswidgetcomponent)
  (bind _ascdplayer_standings_widget (Utilities|Casting|CastToCDPlayerStandingsWidget (UserInterface|GetUserWidgetObject _rankingswidgetcomponent)))
  (Variables|Default|SetRankingsPanel _ascdplayer_standings_widget)
  (bind _ascdgame_instance (Utilities|Casting|CastToCDGameInstance (Game|GetGameInstance)))
  (bind _returnvalue (Class|CDGameInstance|GetGlobalMenuPanelManager _ascdgame_instance))
  (Class|CDMenuPanelManager|Instantiate _returnvalue self))

(event MouseInput|EventActorEndCursorOver
  (Variables|Default|SetCursorOver false))

(fn ConstructionScript)