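; MenuHover is an actor that drives a virtual cursor across 3D widget menu panels using mouse, keyboard or gamepad.
; Each tick, unless camera control is active, it moves, then feeds a custom line trace to WidgetInteraction, which also receives select and scroll input.
; Hits align the cursor to flat or cylindrical surfaces and update the panel manager's nearest boundary.
; Misses jump to the adjacent panel through that boundary or restore the last valid position.
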(event EventTick
  (params (DeltaSeconds :type Float%20%28single-precision%29))
  (Variables|Default|SetDeltaTime DeltaSeconds)
  (bind _ascdmenu_pawn (Utilities|Casting|CastToCDMenuPawn (Game|Player|GetPlayerPawn 0)))
  (if (Variables|/Script/ProjectCore.CDBaseCamera|GetCamControl (Variables|/Script/ProjectCore.CDMenuPawn|GetCamera _ascdmenu_pawn))
    ;[1 1 1] Keep location in same place if cam control active
    (Transformation|SetActorLocation (Variables|Default|GetLastGlobalLocation) false false)
    (else
      ;[1 1 1] Must move based on user input before performing the hit trace; otherwise, the hit trace result will be one frame behind.
      (bind _returnvalue (CallFunction|GetVerticalInput))
      (bind _outputpin (CallFunction|GetHorizontalInput))
      (Transformation|SetActorLocation (+ (+ (Transformation|GetActorLocation) (* (Transformation|GetActorUpVector) _returnvalue)) (* (Transformation|GetActorRightVector) _outputpin)) false false)
      ;[1 1 1] Using custom hit trace. NOTE: In order for this work, WidgetInteraction source has to be "custom"
      (bind _hit_result (CallFunction|DoTraceandGetHitResult (Transformation|GetActorTransform)))
      (Class|WidgetInteractionComponent|SetCustomHitResult (Variables|Default|GetWidgetInteraction) _hit_result)
      (Utilities|IsValid (.HitComponent (Collision|BreakHitResult _hit_result))
        (:Is%20Valid
          (if (.bBlockingHit (Collision|BreakHitResult _hit_result))
            (bind _aswidget_component (Utilities|Casting|CastToWidgetComponent (.HitComponent (Collision|BreakHitResult _hit_result)))
              (:then
                (Variables|Default|SetLastWidgetComponent _aswidget_component)
                (if (Variables|Default|GetbSetOnce)
                  _
                  (else
                    (Rendering|SetVisibility (Variables|Default|GetCursorImage) true true) ; So we dont start with cursor enabled until\nconditions are met (we hit the menu with\nour mourse/controller)
                    (Variables|Default|SetbSetOnce true)))
                ;[1 1 1] Sets variables that will be used for the menu panel movement and accessed when can no longer move in a specific direction.
                (Variables|Default|SetRawHitPoint (.ImpactPoint (Collision|BreakHitResult _hit_result)))
                (Variables|Default|SetLastLocCursor (Transformation|GetWorldLocation (Variables|Default|GetCursorAnchor)))
                (Variables|Default|SetLastGlobalLocation (Transformation|GetActorLocation))
                (Variables|Default|SetLastRot (Transformation|GetActorRotation))
                (Variables|Default|SetLast%20Rot%20Cursor (Transformation|GetWorldRotation (Variables|Default|GetCursorRotationAnchor)))
                ;[1 0.916 0.926] Jakob set correct cursor rotation based on normal of surface
                (CallFunction|SetCursorLocationandRotation _hit_result)
                (bind _ascdgame_instance (Utilities|Casting|CastToCDGameInstance (Game|GetGameInstance)))
                (bind _returnvalue_2 (Class|CDGameInstance|GetGlobalMenuPanelManager _ascdgame_instance))
                (Class|CDMenuPanelManager|GetMenuPanelfromWidget _returnvalue_2 (Variables|Default|GetLastWidgetComponent))
                (bind _output_get (Variables|Default|SetCurrentSign (Class|CDMenuPanelManager|SideOfLine _returnvalue_2 (Variables|Default|GetRawHitPoint))))
                ;[1 1 1] We use a "point in triangle" method to find the nearest boundary well before we need to travel there.
                (bind _ascdgame_instance_2 (Utilities|Casting|CastToCDGameInstance (Game|GetGameInstance)))
                (bind _returnvalue_3 (Class|CDGameInstance|GetGlobalMenuPanelManager _ascdgame_instance_2))
                (Class|CDMenuPanelManager|FindNearestBoundary _returnvalue_3 (Variables|Default|GetLastWidgetComponent) (Variables|Default|GetRawHitPoint)))
              (:CastFailed
                ;[1 1 1] If no hit in this direction, set the location and rotation of the cursor to what it was before and keeps it in place. Also will handle menu panel movement. if there is a boundary it can head to
                (if (Math|Vector|NotEqual(Vector) (Variables|Default|GetLastGlobalLocation) "0, 0, 0" 0.0001) :!label _label
                  (if (Utilities|Enum|NotEqual(Enum) (Variables|/Script/ProjectCore.CDMenuPanelManager|GetBoundaryEntryDir _returnvalue_3) "NONE")
                    (bind _returnvalue_4 (Class|CDMenuPanelManager|MovetoNextPanel _returnvalue_3 (Math|Transform|MakeTransform (Variables|Default|GetLastGlobalLocation) (Variables|Default|GetLastRot) (Transformation|GetActorScale3D)) (Variables|Default|GetLastWidgetComponent))) ; NOTE: Prepares the movement, doesn't actually move. Calls HitTarget function.
                    (bind _output_get_2 (Variables|Default|SetNewTransform _returnvalue_4))
                    (if (Variables|Default|GetbHitBoundary)
                      ;[1 1 1] Actually performs the movement. and moves the cursor from current panel to next active panel.
                      (Transformation|SetActorTransform _output_get_2)
                      (Development|PrintString (Utilities|String|Append "New Transform Rotation = " (Utilities|String|ToString(Rotator) (.rotation (Variables|Default|GetNewTransform)))) false false "(R=1.000000,G=0.000000,B=0.269072,A=1.000000)" 5.0)
                      (bind _hit_result_2 (CallFunction|DoTraceandGetHitResult (Transformation|GetActorTransform)))
                      (Utilities|Casting|CastToWidgetComponent (.HitComponent (Collision|BreakHitResult _hit_result_2))
                        (:then
                          (Transformation|SetWorldRotation (Variables|Default|GetWidgetInteraction) (Math|Conversions|RotationFromXVector (Math|Vector|NegateVector (.ImpactNormal (Collision|BreakHitResult _hit_result_2)))) false false)
                          (CallFunction|SetCursorLocationandRotation _hit_result_2))
                        (:CastFailed
                          (Development|PrintString (Utilities|String|Append "ERROR in MenuHover::EventGraph, while moving cursor to next widget: Failed to cast HitResult to a WidgetComponent. Result object is: " (Utilities|GetObjectName (.HitComponent (Collision|BreakHitResult _hit_result_2))) ". Will reset to LastGlobalLocation/LastRot.") true true "(R=1.000000,G=0.000000,B=0.000000,A=1.000000)")
                          (Transformation|SetActorLocation (Variables|Default|GetLastGlobalLocation) false false :!label _label_2)
                          (Transformation|SetActorRotation (Variables|Default|GetLastRot))))
                      (else
                        (goto _label_2)))
                    (else
                      (goto _label_2))))))
            (else
              (goto _label))))
        (:Is%20Not%20Valid
          (goto _label))))))

(event EventBeginPlay
  ;[1 1 1] One time enable input for widget interaction component to work and setup the distance mouse cursor is from the menu
  (Components|Activation|SetActive (Variables|Default|GetWidgetInteraction) true false)
  (Input|EnableInput (Game|GetPlayerController 0))
  (bind _returnvalue (Actor|GetActorOfClass "/Game/Blueprints/MenuWidgets/BP_MainMenu.BP_MainMenu_C"))
  (Class|CDMenuApproximationActor|ExtractMenuPosition (Variables|/Game/Blueprints/MenuWidgets/BP_MainMenu.BP_MainMenu_C|GetLeftWidgetComponent _returnvalue) (Variables|Default|GetCursorImage) true))

(event Input|ActionEvents|InputActionMenuSelect
  (params (Key :type Key%20Structure :default "None"))
  ;[1 1 1] This is what works for touch controllers + some other unconvential inputs (enter)
  (:Pressed
    (Class|WidgetInteractionComponent|PressPointerKey (Variables|Default|GetWidgetInteraction) "LeftMouseButton"))
  (:Released
    (Class|WidgetInteractionComponent|ReleasePointerKey (Variables|Default|GetWidgetInteraction) "LeftMouseButton")))

(event Input|MouseEvents|MouseWheelAxis
  (params (AxisValue :type Float%20%28single-precision%29))
  (Class|WidgetInteractionComponent|ScrollWheel (Variables|Default|GetWidgetInteraction) AxisValue))

(fn ConstructionScript)

(fn SetCursorLocationandRotation
  (params (Hit%20Result :type Hit%20Result%20Structure%20%28by%20ref%29))
  (bind (_bblockinghit _binitialoverlap _time _distance _location _impactpoint _normal _impactnormal _physmat _hitactor _hitcomponent) (Collision|BreakHitResult Hit%20Result))
  (bind _distancefrompanel (Variables|Default|GetDistanceFromPanel))
  (bind _cursorrelativeoffset (Variables|Default|GetCursorRelativeOffset))
  (bind _cursorrotationanchor (Variables|Default|GetCursorRotationAnchor))
  (bind _returnvalue (* _normal _distancefrompanel))
  (bind _returnvalue_2 (+ _cursorrelativeoffset _impactpoint _returnvalue))
  ;[1 1 1] The correct cylindrical depth will debug as a yellow line and where we can calculate the most correct impact normal
  (bind _aswidget_component (Utilities|Casting|CastToWidgetComponent _hitcomponent)
    (:then
      (bind _returnvalue_3 (Class|CDMenuApproximationActor|GetCorrectCylindricalDepth _location _aswidget_component))
      (switch Utilities|FlowControl|Switch|SwitchonEWidgetGeometryMode (Class|WidgetComponent|GetGeometryMode _aswidget_component)
        (:Plane
          (Transformation|SetWorldRotation _cursorrotationanchor (Math|Rotator|FindLookatRotation _impactpoint (+ _impactpoint (* _normal 1.0))) false false))
        (:Cylinder
          (Transformation|SetWorldRotation _cursorrotationanchor (Math|Rotator|FindLookatRotation _impactpoint (+ _impactpoint (* (* _returnvalue_3 -1.0) 1))) false false)))
      ;[1 1 1] Sets location. Rotation must be set first! (Otherwise, the cursor lags behind by one frame.)
      (Transformation|SetWorldLocation (Variables|Default|GetCursorAnchor) _returnvalue_2 false false)
      (Development|PrintString (Utilities|String|Append "Cursor Location Set to: " (Utilities|String|ToString(Vector) _returnvalue_2)) false false "(R=0.000000,G=0.660000,B=1.000000,A=1.000000)" (Variables|Default|GetDeltaTime))
      (return))
    (:CastFailed
      (Development|PrintString "ERROR In MenuHover::SetCursorLocationAndRotation: failed to cast  HitResult.HitComponent to WidgetComponent!" true true "(R=1.000000,G=0.000000,B=0.000000,A=1.000000)"))))

(fn SetPanelBounds
  (params (Target :type CD%20Menu%20Panel%20Object%20Reference))
  (Variables|Default|SetTopVertBound (Variables|/Script/ProjectCore.CDMenuPanel|GetTopVertBound Target))
  (Variables|Default|SetBotVertBound (Variables|/Script/ProjectCore.CDMenuPanel|GetBotVertBound Target))
  (Variables|Default|SetLeftHozBound (Variables|/Script/ProjectCore.CDMenuPanel|GetLeftHozBound Target))
  (Variables|Default|SetRightHozBound (Variables|/Script/ProjectCore.CDMenuPanel|GetRightHozBound Target))
  (Variables|Default|SetCurrentPanelCenter (Variables|/Script/ProjectCore.CDMenuPanel|GetCenter Target)))

(fn GetVerticalInput
  (bind _returnvalue (Game|GetPlayerController 0))
  (bind _currentpanelcenter (Variables|Default|GetCurrentPanelCenter))
  (bind _cursoranchor (Variables|Default|GetCursorAnchor))
  (bind _returnvalue_2 (Transformation|GetWorldLocation _cursoranchor))
  (bind _returnvalue_3 (Subsystems|GetCDLocalPlayerSubsystem _returnvalue))
  (bind _returnvalue_4 (- (.z _returnvalue_2) (.z _currentpanelcenter)))
  (Utilities|IsValid _returnvalue_3
    (:Is%20Valid
      (bind _returnvalue_5 (Class|CDLocalPlayerSubsystem|GetCustomMouseSensitivity _returnvalue_3))
      (Development|PrintString (Utilities|String|ToString(Float) (* (.DeltaY (Class|PlayerController|GetInputMouseDelta _returnvalue)) _returnvalue_5)) true false "(R=0.000000,G=0.660000,B=1.000000,A=1.000000)" (Variables|Default|GetDeltaTime))
      (Development|PrintString (Utilities|String|Append "Mouse delta Y: " (Utilities|String|ToString(Float) (* (Input|AxisValues|GetMenu_Vertical) (Variables|Default|GetDeltaTime) (Variables|Default|GetVertSpeed)))) true false "(R=0.000000,G=0.660000,B=1.000000,A=1.000000)" (Variables|Default|GetDeltaTime))
      (switch Utilities|FlowControl|Switch|SwitchonESwitcherooInputDevice (Class|SwitcherooBlueprintLibrary|GetDetectedInputDevice)
        (:KeyboardMouse
          (Variables|Default|SetVertSpeed 1e+01))
        (:Gamepad
          (Variables|Default|SetVertSpeed 4e+01)))
      (if (or (> (Math|Float|Absolute(Float) (* (.DeltaY (Class|PlayerController|GetInputMouseDelta _returnvalue)) _returnvalue_5)) 0.0) (> (Math|Float|Absolute(Float) (* (Input|AxisValues|GetMenu_Vertical) (Variables|Default|GetDeltaTime) (Variables|Default|GetVertSpeed))) 0.1))
        (bind _output_get (LocalVariables|SetChangeInY (- (+ _returnvalue_4 (* (.DeltaY (Class|PlayerController|GetInputMouseDelta _returnvalue)) _returnvalue_5) (* (Input|AxisValues|GetMenu_Vertical) (Variables|Default|GetDeltaTime) (Variables|Default|GetVertSpeed))) _returnvalue_4)))
        (else
          (LocalVariables|SetChangeInY 0.0)))
      (return _output_get))))

(fn GetHorizontalInput
  (bind _returnvalue (Game|GetPlayerController 0))
  (bind _currentpanelcenter (Variables|Default|GetCurrentPanelCenter))
  (bind _cursoranchor (Variables|Default|GetCursorAnchor))
  (bind _returnvalue_2 (Transformation|GetWorldLocation _cursoranchor))
  (bind _returnvalue_3 (Subsystems|GetCDLocalPlayerSubsystem _returnvalue))
  (bind _returnvalue_4 (- (.x _returnvalue_2) (.x _currentpanelcenter)))
  (Utilities|IsValid _returnvalue_3
    (:Is%20Valid
      (bind _returnvalue_5 (Class|CDLocalPlayerSubsystem|GetCustomMouseSensitivity _returnvalue_3))
      (Development|PrintString (Utilities|String|ToString(Float) (* (Input|AxisValues|GetMenu_Horizontal) (Variables|Default|GetDeltaTime) (Variables|Default|GetHozSpeed))) true false "(R=0.000000,G=0.660000,B=1.000000,A=1.000000)" (Variables|Default|GetDeltaTime))
      (Development|PrintString (Utilities|String|Append "Mouse delta: " (Utilities|String|ToString(Float) (* (.DeltaX (Class|PlayerController|GetInputMouseDelta _returnvalue)) _returnvalue_5))) true false "(R=0.000000,G=0.660000,B=1.000000,A=1.000000)" (Variables|Default|GetDeltaTime))
      (switch Utilities|FlowControl|Switch|SwitchonESwitcherooInputDevice (Class|SwitcherooBlueprintLibrary|GetDetectedInputDevice)
        (:KeyboardMouse
          (Variables|Default|SetHozSpeed 1e+01))
        (:Gamepad
          (Variables|Default|SetHozSpeed 6e+01)))
      (if (or (> (Math|Float|Absolute(Float) (* (.DeltaX (Class|PlayerController|GetInputMouseDelta _returnvalue)) _returnvalue_5)) 0.0) (> (Math|Float|Absolute(Float) (* (Input|AxisValues|GetMenu_Horizontal) (Variables|Default|GetDeltaTime) (Variables|Default|GetHozSpeed))) 0.1))
        (bind _output_get (LocalVariables|SetChangeInX (- (+ _returnvalue_4 (* (.DeltaX (Class|PlayerController|GetInputMouseDelta _returnvalue)) _returnvalue_5) (* (Input|AxisValues|GetMenu_Horizontal) (Variables|Default|GetDeltaTime) (Variables|Default|GetHozSpeed))) _returnvalue_4)))
        (else
          (LocalVariables|SetChangeInX 0.0)))
      (return _output_get))))

(fn HitTarget
  (params (InTransform :type Transform))
  (bind _hit_result (CallFunction|DoTraceandGetHitResult InTransform))
  (bind _aswidget_component (Utilities|Casting|CastToWidgetComponent (.HitComponent (Collision|BreakHitResult _hit_result)))
    (:then
      (LocalVariables|SetFoundPanel (Math|Transform|MakeTransform (.ImpactPoint (Collision|BreakHitResult _hit_result)) (Variables|Default|GetLastRot) "1,1,1"))
      (Variables|Default|SetbHitBoundary (Utilities|IsValid _aswidget_component)))
    (:CastFailed
      (Development|PrintString (Utilities|String|Append "Cast HitComponent As WidgetComponent failed in MenuHover::HitTarget. HitComponent is: " (Utilities|GetObjectName (.HitComponent (Collision|BreakHitResult _hit_result)))))
      (LocalVariables|SetFoundPanel (Math|Transform|MakeTransform "0, 0, 0"))
      (Variables|Default|SetbHitBoundary false)))
  (return (LocalVariables|GetFoundPanel)))

(fn DoTraceandGetHitResult
  (params (Current%20Transform :type Transform))
  (bind _outhit (Collision|LineTraceForObjects (.location Current%20Transform) (+ (.location Current%20Transform) (* (Class|CDMenuApproximationActor|GetCorrectForwardVector (.rotation Current%20Transform)) (Variables|/Script/UMG.WidgetInteractionComponent|GetInteractionDistance (Variables|Default|GetWidgetInteraction)))) (Variables|Default|GetHitWidgetQuery) false 0 (Variables|Default|GetDoDebug) false "(R=1.000000,G=0.000000,B=0.000000,A=1.000000)" "(R=0.278447,G=0.000000,B=1.000000,A=1.000000)"))
  (return _outhit))