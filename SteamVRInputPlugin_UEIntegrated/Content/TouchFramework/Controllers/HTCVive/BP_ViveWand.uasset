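; BP_ViveWand is the HTC Vive wand controller in a touch framework, driving a HandActor for a virtual hand.
; Each tick it sets thumb and index poses, and on input focus changes it activates or deactivates the hand, unhiding itself when focus is lost.
; Left/right-filtered chains for grab, release and index actions are present, but no event runs them.
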(event EventTick
  (params (DeltaSeconds :type Float%20%28single-precision%29))
  (bind _returnvalue (Class|OculusFunctionLibrary|HasInputFocus))
  (bind _handactor (Variables|Default|GetHandActor))
  (|CallParentFunction DeltaSeconds)
  (Utilities|FlowControl|Sequence
    (:then_0
      (CallFunction|UpdateHandAnimations))
    (:then_1
      (if (Math|Boolean|NotEqual(Boolean) (Variables|Default|GetInputFocus) _returnvalue)
        (bind _output_get (Variables|Default|SetInputFocus _returnvalue))
        (if _output_get
          (Default|ActivateHand _handactor)
          (else
            (Rendering|SetActorHiddenInGame false)
            (Default|DeactivateHand _handactor)))))))

(fn ConstructionScript
  (|CallParentFunction))

(fn UpdateHandAnimations
  (Default|UpdateHandAnimation (Variables|Default|GetHandActor) 0.6 0.55 0.0 0.0 0.0))