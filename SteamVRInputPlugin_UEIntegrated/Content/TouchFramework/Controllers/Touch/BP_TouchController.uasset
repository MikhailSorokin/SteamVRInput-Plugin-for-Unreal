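; VR Touch controller for one hand, showing the matching left or right controller model and driving its HandActor.
; Hand-filtered key events set button states and forward trigger, face button and grip input as index, thumb and grab actions.
; Tick polls axes for animation values, finger poses and thumbstick-angle teleport rotation, and toggles the hand on input focus changes.
; Laser toggle and thumbstick teleport activation are present but inactive.
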(event EventSetControllerType
  (params (New%20Type :type EControllerHand%20Enum :default "Left"))
  (bind _controller (Variables|Default|GetController))
  (|CallParentFunction New%20Type)
  (switch Utilities|FlowControl|Switch|SwitchonEControllerHand New%20Type
    (:Left
      (Class|SkinnedMeshComponent|SetSkeletalMesh _controller "/Game/TouchFramework/Controllers/Touch/Models/SK_left_touch_controller_model_skel.SK_left_touch_controller_model_skel" true)
      (Components|SkeletalMesh|SetAnimInstanceClass _controller "/Game/TouchFramework/Controllers/Touch/Models/ABP_LeftTouchAnimBP.ABP_LeftTouchAnimBP_C"))
    (:Right
      (Class|SkinnedMeshComponent|SetSkeletalMesh _controller "/Game/TouchFramework/Controllers/Touch/Models/SK_right_touch_controller_model_skel.SK_right_touch_controller_model_skel" true)
      (Components|SkeletalMesh|SetAnimInstanceClass _controller "/Game/TouchFramework/Controllers/Touch/Models/ABP_RightTouchAnimBP.ABP_RightTouchAnimBP_C"))))

(event EventTick
  (params (DeltaSeconds :type Float%20%28single-precision%29))
  (bind _returnvalue (Class|OculusFunctionLibrary|HasInputFocus))
  (bind _handactor (Variables|Default|GetHandActor))
  (|CallParentFunction DeltaSeconds)
  (Utilities|FlowControl|Sequence
    (:then_0
      (CallFunction|UpdateAnimationValues)
      (CallFunction|UpdateHandAnimations)
      (CallFunction|UpdateTeleportRotation))
    (:then_1
      (if (Math|Boolean|NotEqual(Boolean) (Variables|Default|GetInputFocus) _returnvalue)
        (bind _output_get (Variables|Default|SetInputFocus _returnvalue))
        (if _output_get
          (Default|ActivateHand _handactor)
          (else
            (Rendering|SetActorHiddenInGame false)
            (Default|DeactivateHand _handactor)))))))

(event EventBeginPlay
  (Input|EnableInput (Game|GetPlayerController 0)))

(event Input|GamepadEvents|GamepadSpecialRight
  (params (Key :type Key%20Structure))
  (:Pressed
    (if false ; do we want a laser?
      (Default|ToggleLaser (Variables|/Game/TouchFramework/Hands/BP_HandBP.BP_HandBP_C|GetMyPawn (Variables|Default|GetHandActor))))))

(event Input|KeyboardEvents|MotionControllerLeftFaceButton1
  (params (Key :type Key%20Structure))
  (bind _handactor (Variables|Default|GetHandActor))
  (bind _hand (Variables|Default|GetHand))
  (bind _returnvalue (Utilities|Enum|Equal(Enum) _hand "Left"))
  (:Pressed
    (if _returnvalue
      (Default|ThumbAction _handactor)))
  (:Released
    (if _returnvalue
      (Default|ThumbActionEnd _handactor))))

(event Input|KeyboardEvents|MotionControllerLeftFaceButton2
  (params (Key :type Key%20Structure))
  (bind _handactor (Variables|Default|GetHandActor))
  (bind _hand (Variables|Default|GetHand))
  (bind _returnvalue (Utilities|Enum|Equal(Enum) _hand "Left"))
  (:Pressed
    (if _returnvalue
      (Default|ThumbAction _handactor)))
  (:Released
    (if _returnvalue
      (Default|ThumbActionEnd _handactor))))

(event Input|KeyboardEvents|MotionControllerRightTrigger
  (params (Key :type Key%20Structure))
  (bind _hand (Variables|Default|GetHand))
  (bind _handactor (Variables|Default|GetHandActor))
  (bind _returnvalue (Utilities|Enum|Equal(Enum) _hand "Right"))
  (:Pressed
    (if _returnvalue
      (Default|IndexAction _handactor)))
  (:Released
    (if _returnvalue
      (Default|IndexActionEnd _handactor))))

(event Input|KeyboardEvents|MotionControllerLeftGrip1
  (params (Key :type Key%20Structure))
  (bind _hand (Variables|Default|GetHand))
  (bind _handactor (Variables|Default|GetHandActor))
  (bind _returnvalue (Utilities|Enum|Equal(Enum) _hand "Left"))
  (:Pressed
    (if _returnvalue
      (Default|AttemptGrab _handactor)))
  (:Released
    (if _returnvalue
      (Default|Release _handactor))))

(event Input|KeyboardEvents|MotionControllerLeftTrigger
  (params (Key :type Key%20Structure))
  (bind _handactor (Variables|Default|GetHandActor))
  (bind _hand (Variables|Default|GetHand))
  (bind _returnvalue (Utilities|Enum|Equal(Enum) _hand "Left"))
  (:Pressed
    (if _returnvalue
      (Default|IndexAction _handactor)))
  (:Released
    (if _returnvalue
      (Default|IndexActionEnd _handactor))))

(event Input|KeyboardEvents|MotionControllerRightGrip1
  (params (Key :type Key%20Structure))
  (bind _hand (Variables|Default|GetHand))
  (bind _handactor (Variables|Default|GetHandActor))
  (bind _returnvalue (Utilities|Enum|Equal(Enum) _hand "Right"))
  (:Pressed
    (if _returnvalue
      (Default|AttemptGrab _handactor)))
  (:Released
    (if _returnvalue
      (Default|Release _handactor))))

(event Input|KeyboardEvents|MotionControllerRightFaceButton1
  (params (Key :type Key%20Structure))
  (bind _hand (Variables|Default|GetHand))
  (bind _returnvalue (Utilities|Enum|Equal(Enum) _hand "Right"))
  (:Pressed
    (if _returnvalue
      (Variables|Default|SetButton1 true)))
  (:Released
    (if _returnvalue
      (Variables|Default|SetButton1 false))))

(event Input|KeyboardEvents|MotionControllerLeftFaceButton1
  (params (Key :type Key%20Structure))
  (bind _hand (Variables|Default|GetHand))
  (bind _returnvalue (Utilities|Enum|Equal(Enum) _hand "Left"))
  (:Pressed
    (if _returnvalue
      (Variables|Default|SetButton1 true)))
  (:Released
    (if _returnvalue
      (Variables|Default|SetButton1 false))))

(event Input|KeyboardEvents|MotionControllerLeftFaceButton2
  (params (Key :type Key%20Structure))
  (bind _hand (Variables|Default|GetHand))
  (bind _returnvalue (Utilities|Enum|Equal(Enum) _hand "Left"))
  (:Pressed
    (if _returnvalue
      (Variables|Default|SetButton2 true)))
  (:Released
    (if _returnvalue
      (Variables|Default|SetButton2 false))))

(event Input|KeyboardEvents|MotionControllerRightFaceButton1
  (params (Key :type Key%20Structure))
  (bind _handactor (Variables|Default|GetHandActor))
  (bind _hand (Variables|Default|GetHand))
  (bind _returnvalue (Utilities|Enum|Equal(Enum) _hand "Right"))
  (:Pressed
    (if _returnvalue
      (Default|ThumbAction _handactor)))
  (:Released
    (if _returnvalue
      (Default|ThumbActionEnd _handactor))))

(event Input|KeyboardEvents|MotionControllerRightFaceButton2
  (params (Key :type Key%20Structure))
  (bind _handactor (Variables|Default|GetHandActor))
  (bind _hand (Variables|Default|GetHand))
  (bind _returnvalue (Utilities|Enum|Equal(Enum) _hand "Right"))
  (:Pressed
    (if _returnvalue
      (Default|ThumbAction _handactor)))
  (:Released
    (if _returnvalue
      (Default|ThumbActionEnd _handactor))))

(event Input|KeyboardEvents|MotionControllerRightFaceButton2
  (params (Key :type Key%20Structure))
  (bind _hand (Variables|Default|GetHand))
  (bind _returnvalue (Utilities|Enum|Equal(Enum) _hand "Right"))
  (:Pressed
    (if _returnvalue
      (Variables|Default|SetButton2 true)))
  (:Released
    (if _returnvalue
      (Variables|Default|SetButton2 false))))

(fn ConstructionScript
  (|CallParentFunction))

(fn UpdateAnimationValues
  (switch Utilities|FlowControl|Switch|SwitchonEControllerHand (Variables|Default|GetHand)
    (:Left
      (Variables|Default|SetThumbstickX (Class|Actor|GetInputAxisKeyValue))
      (Variables|Default|SetThumbstickY (Class|Actor|GetInputAxisKeyValue))
      (Variables|Default|SetTriggerAxis (Class|Actor|GetInputAxisKeyValue))
      (Variables|Default|SetGripAxis (Class|Actor|GetInputAxisKeyValue)))
    (:Right
      (Variables|Default|SetThumbstickX (Class|Actor|GetInputAxisKeyValue))
      (Variables|Default|SetThumbstickY (Class|Actor|GetInputAxisKeyValue))
      (Variables|Default|SetTriggerAxis (Class|Actor|GetInputAxisKeyValue))
      (Variables|Default|SetGripAxis (Class|Actor|GetInputAxisKeyValue)))))

(fn UpdateHandAnimations
  (switch Utilities|FlowControl|Switch|SwitchonEControllerHand (Variables|Default|GetHand)
    (:Left
      (Default|UpdateHandAnimation (Variables|Default|GetHandActor) (Math|Float|Clamp(Float) (Class|Actor|GetInputAxisKeyValue) 0.5) (Math|Float|Clamp(Float) (Class|Actor|GetInputAxisKeyValue) 0.6) (Math|Float|Clamp(Float) (* (- 1.0 (Class|Actor|GetInputAxisKeyValue)) 0.75) 0.4 0.5) 0.4 0.4))
    (:Right
      (Default|UpdateHandAnimation (Variables|Default|GetHandActor) (Math|Float|Clamp(Float) (Class|Actor|GetInputAxisKeyValue) 0.5) (Math|Float|Clamp(Float) (Class|Actor|GetInputAxisKeyValue) 0.6) (Math|Float|Clamp(Float) (* (- 1.0 (Class|Actor|GetInputAxisKeyValue)) 0.75) 0.4 0.5) 0.4 0.4))))

(fn UpdateTeleportRotation
  (bind _hand (Variables|Default|GetHand))
  (bind _returnvalue (Utilities|Enum|Equal(Enum) _hand "Right"))
  (if (or (Utilities|Enum|Equal(Enum) _hand "Left") _returnvalue)
    (Default|AddTeleportRotation (Variables|Default|GetHandActor) (select _returnvalue (Class|KismetMathLibrary|DegAtan2 (Class|Actor|GetInputAxisKeyValue) (* (Class|Actor|GetInputAxisKeyValue) -1.0)) (Class|KismetMathLibrary|DegAtan2 (Class|Actor|GetInputAxisKeyValue) (* (Class|Actor|GetInputAxisKeyValue) -1.0))))))